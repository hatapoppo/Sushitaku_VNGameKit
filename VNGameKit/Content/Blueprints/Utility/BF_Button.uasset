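; Blueprint function library of shared button feedback for in-game and UI widgets.
; Separate press functions for in-game, UI and cancel buttons each play their own 2D sound and slightly shrink the passed widget, while Released restores its scale.
; Hover only plays a sound.
; Each sound's volume is scaled by the SE volume setting in BP_GameInstance's GlobalData, so a failed cast skips that function's feedback entirely.
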(fn `HoveredUIButton`
  (params (ResizeWidget :type "Widget Object Reference"))
  (bind _asbp_game_instance (cast `/Game/Blueprints/Core/BP_GameInstance` (`GameplayStatics.GetGameInstance` null)))
  (bind _returnvalue (`GameplayStatics.SpawnSound2D` null "/Game/Sounds/決定ボタンを押す7.決定ボタンを押す7" 1.0 1.0 0.0 null))
  (`AudioComponent.AdjustVolume` _returnvalue 0.0 (/ (`/Game/Data/BP_GlobalSave.SE_Volume` (`/Game/Blueprints/Core/BP_GameInstance.GlobalData` _asbp_game_instance)) 100.0) "Linear"))

(fn `PressedCancelButton`
  (params (ResizeWidget :type "Widget Object Reference"))
  (bind _asbp_game_instance (cast `/Game/Blueprints/Core/BP_GameInstance` (`GameplayStatics.GetGameInstance` null)))
  (bind _returnvalue (`GameplayStatics.SpawnSound2D` null "/Game/Sounds/キャンセル6.キャンセル6" 1.0 1.0 0.0 null))
  (`AudioComponent.AdjustVolume` _returnvalue 0.0 (/ (`/Game/Data/BP_GlobalSave.SE_Volume` (`/Game/Blueprints/Core/BP_GameInstance.GlobalData` _asbp_game_instance)) 100.0) "Linear")
  (`/Engine/EditorBlueprintResources/StandardMacros.IsValid` ResizeWidget
    (:`Is Valid`
      (`Widget.SetRenderScale` ResizeWidget (0.9 0.9)))))

(fn `PressedInGameButton`
  (params (ResizeWidget :type "Widget Object Reference"))
  (bind _asbp_game_instance (cast `/Game/Blueprints/Core/BP_GameInstance` (`GameplayStatics.GetGameInstance` null)))
  (bind _returnvalue (`GameplayStatics.SpawnSound2D` null "/Game/Sounds/カーソル移動12.カーソル移動12" 1.0 1.0 0.0 null))
  (`AudioComponent.AdjustVolume` _returnvalue 0.0 (/ (`/Game/Data/BP_GlobalSave.SE_Volume` (`/Game/Blueprints/Core/BP_GameInstance.GlobalData` _asbp_game_instance)) 100.0) "Linear")
  (`/Engine/EditorBlueprintResources/StandardMacros.IsValid` ResizeWidget
    (:`Is Valid`
      (`Widget.SetRenderScale` ResizeWidget (0.9 0.9)))))

(fn `PressedUIButton`
  (params (ResizeWidget :type "Widget Object Reference"))
  (bind _asbp_game_instance (cast `/Game/Blueprints/Core/BP_GameInstance` (`GameplayStatics.GetGameInstance` null)))
  (bind _returnvalue (`GameplayStatics.SpawnSound2D` null "/Game/Sounds/決定ボタンを押す3.決定ボタンを押す3" 1.0 1.0 0.0 null))
  (`AudioComponent.AdjustVolume` _returnvalue 0.0 (/ (`/Game/Data/BP_GlobalSave.SE_Volume` (`/Game/Blueprints/Core/BP_GameInstance.GlobalData` _asbp_game_instance)) 100.0) "Linear")
  (`/Engine/EditorBlueprintResources/StandardMacros.IsValid` ResizeWidget
    (:`Is Valid`
      (`Widget.SetRenderScale` ResizeWidget (0.9 0.9)))))

(fn `Released`
  (params (ResizeWidget :type "Widget Object Reference"))
  (`/Engine/EditorBlueprintResources/StandardMacros.IsValid` ResizeWidget
    (:`Is Valid`
      (`Widget.SetRenderScale` ResizeWidget (1.0 1.0)))))