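; BFL_String is a string utility library whose ConvertCleanText function prepares raw text containing page tags and variable placeholders.
; It trims the text, merges line breaks adjacent to next-page tags into those tags, then replaces the remaining line-break markers.
; A regex then extracts curly-brace variable names, substituting values from BP_GameInstance's GetStatusValue and leaving unknown names untouched.
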(fn `ConvertCleanText`
  (params (Text :type String))
  (returns (ReturnText :type String))
  (locals (TagNextPage :type String :default "<p>") (Indention :type String :default "\\n") (TagPlayerName :type String :default "{PlayerName}") (TagFormula :type String :default "{Formula}") (TagSum :type String :default "{Sum}") (TagDetail :type String :default "{Detail}") (ResultText :type String) (Return :type String) (GameInstance :type "/Game/Blueprints/Core/BP_GameInstance Object Reference"))
  (bind _return (`local.Return`))
  (bind _asbp_game_instance (cast `/Game/Blueprints/Core/BP_GameInstance` (`GameplayStatics.GetGameInstance` null)))
  (set `local.GameInstance` _asbp_game_instance)
  (`|ExecutionSequence`
    (:`then_0`
      (set `local.Return` (`KismetStringLibrary.Replace` (`KismetStringLibrary.Replace` (`KismetStringLibrary.Replace` (`KismetStringLibrary.Trim` Text) (`KismetStringLibrary.Concat_StrStr` (`local.TagNextPage`) (`local.Indention`)) (`local.TagNextPage`)) (`KismetStringLibrary.Concat_StrStr` (`local.Indention`) (`local.TagNextPage`)) (`local.TagNextPage`)) (`local.Indention`) " \n")))
    (:`then_1`
      ; 変数名を値に変換
      (set `local.ResultText` _return)
      (for _array_element (`Utility.ExtractPattern` _return "\\{(.*?)\\}")
        (bind (_value _exist) (`/Game/Blueprints/Core/BP_GameInstance.GetStatusValue` (`local.GameInstance`) _array_element))
        (if _exist
          (set `local.ResultText` (`KismetStringLibrary.Replace` (`local.ResultText`) (`KismetStringLibrary.Concat_StrStr` "{" _array_element "}") _value)))))
    (:`then_2`
      (return (`local.ResultText`)))))